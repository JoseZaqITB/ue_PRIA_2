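; Game state for a Red-versus-Blue match, driving preparing, playing and finished phases and picking connection or in-game UI on BeginPlay.
; Tick counts down preparation, then play time; Red wins on timeout, Blue through MakeBlueWin.
; FinishGame unpossesses players, passes remaining play time to winners' controllers as a best time, then server-travels to restart the level after a delay.
; Kill-limit win checks are left unwired.
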(event `self.ReceiveBeginPlay`
  (bind _returnvalue (`GameplayStatics.GetGameMode`))
  (`/Engine/EditorBlueprintResources/StandardMacros.IsValid` _returnvalue ; si es valido, es porque ya estoy conectado a un servidor
    (:`Is Valid`
      (if (`KismetStringLibrary.EqualEqual_StrStr` (`GameModeBase.OptionsString` _returnvalue))
        (bind _returnvalue_2 (`|CreateWidget` "/Game/MINE/UI/ui_conection.ui_conection_C"))
        (`UserWidget.AddToViewport` _returnvalue_2 0)
        (else
          (bind _returnvalue_3 (`|CreateWidget` "/Game/MINE/UI/UI_InGame.UI_InGame_C" :!label _label))
          (`UserWidget.AddToViewport` _returnvalue_3 0))))
    (:`Is Not Valid`
      (goto _label))))

(event `FinishGame`
  (set `self.partidaState` "NewEnumerator2") ; terminar partida
  (bind _result (`/Engine/EditorBlueprintResources/StandardMacros.DecrementInt` (`GameplayStatics.GetNumPlayerControllers`))
    (:`  `
      ;[1 1 1] inhabilitar a los jugadores controlar su personaje
      (for _index (range (+ _result 1))
        (bind _returnvalue (`GameplayStatics.GetPlayerController` _index))
        (`Controller.UnPossess` _returnvalue)
        ;[1 1 1] playfab: añadir el mejor tiempo del jugador en caso de que sea el ganador y haya hecho mejor tiempo en esta partida
        (bind _asbp_my_player_controller (cast `/Game/MINE/BP_myPlayerController` _returnvalue))
        (bind _asbp_my_player_state (cast `/Game/MINE/BP_myPlayerState` (`Controller.PlayerState` _asbp_my_player_controller)))
        (if (`|EnumEquality` (`self.winner`) (`/Game/MINE/BP_myPlayerState.team` _asbp_my_player_state))
          (`/Game/MINE/BP_myPlayerController.UpdateBestWinTime` _asbp_my_player_controller (`self.playDuration`))))
      ;[1 1 1] reiniciar partida despues de 5seg
      (`KismetSystemLibrary.Delay` 5.0)
      (bind _returnvalue_2 (`GameplayStatics.GetCurrentLevelName` true))
      (`KismetSystemLibrary.ExecuteConsoleCommand` (`KismetStringLibrary.Concat_StrStr` "serverTravel " _returnvalue_2) null))))

(event `PrepareGame`
  (set `self.partidaState` "NewEnumerator3") ; actualiza el estado partida  a preparando
)

(event `StartGame`
  (set `self.partidaState` "NewEnumerator1") ; actualiza el estado partida  a empezada
)

(event `self.ReceiveTick`
  (params (DeltaSeconds :type "Float (single-precision)"))
  ;[1 1 1] countDown para el esrado preparing
  (if (`|EnumEquality` (`self.partidaState`) "NewEnumerator3")
    (bind _updatetime (`self.CoundDown` (`self.prepareCountDown`)))
    (bind _output_get (set `self.prepareCountDown` _updatetime))
    (if (<= _output_get 0.0)
      (`self.StartGame`))
    (else
      ;[1 1 1] Al pasar 2min el equipo red gana
      (if (`|EnumEquality` (`self.partidaState`) "NewEnumerator1")
        (bind _updatetime_2 (`self.CoundDown` (`self.playDuration`)))
        (bind _output_get_2 (set `self.playDuration` _updatetime_2))
        (if (<= _output_get_2 0.0)
          (set `self.winner` "NewEnumerator0")
          (`self.FinishGame`))))))

(event `MakeBlueWin`
  (set `self.winner` "NewEnumerator1")
  (`self.FinishGame`))

(fn `CoundDown`
  (params (time :type "Float (double-precision)"))
  (returns (updateTime :type "Float (double-precision)"))
  (return (- time (`GameplayStatics.GetWorldDeltaSeconds`))))

(fn `OnRep_iniTime`)

(fn `UserConstructionScript`)